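; BP_Mutant is a melee enemy that chases the player and attacks with its arm.
; Once activated, a looping timer drives AI movement toward the player and flags attacking on arrival; Tick then keeps it yawed at the player.
; A socket-attached arm hitbox, initially collisionless, calls GetHit on the character's capsule and sets HasBounced if that returns true.
; On death, capsule collision is disabled and the mesh ragdolls.
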(event `self.ReceiveBeginPlay`
  (`parent.ReceiveBeginPlay`)
  (`KismetSystemLibrary.K2_SetTimerDelegate` (delegate `Think`) 0.4 true))

(event `Think`
  (if (`self.isActivated?`)
    (if (not (`self.isAttacking?`))
      (`|AIMoveTo` self (0.0 0.0 0.0) (`GameplayStatics.GetPlayerPawn` 0) 200.0
        (:`OnSuccess`
          (set `self.isAttacking?` true))))))

(event `self.ArmHitbox.OnComponentBeginOverlap`
  (params (OverlappedComponent :type "PrimitiveComponent Object Reference") (OtherActor :type "Actor Object Reference") (OtherComp :type "PrimitiveComponent Object Reference") (OtherBodyIndex :type Integer) (bFromSweep :type Boolean) (SweepResult :type "HitResult Structure (by ref)"))
  (cast `CapsuleComponent` OtherComp)
  (bind _asbp_character (cast `/Game/mobs/character/BP_Character` OtherActor))
  (bind _wasblocked (`/Game/mobs/character/BP_Character.GetHit` _asbp_character))
  (if _wasblocked
    (set `self.hasBounced?` true)))

(event `self.ReceiveTick`
  (params (DeltaSeconds :type "Float (single-precision)"))
  (bind (_returnvalue_roll _returnvalue_pitch _returnvalue_yaw) (`KismetMathLibrary.BreakRotator` (`KismetMathLibrary.FindLookAtRotation` (`self.K2_GetActorLocation`) (`self.K2_GetActorLocation` (`GameplayStatics.GetPlayerPawn` 0)))))
  (if (and (`self.isAttacking?`) (not (`self.isDying?`)))
    (`SceneComponent.K2_SetWorldRotation` (`self.CapsuleComponent`) (`KismetMathLibrary.MakeRotator` 0.0 0.0 _returnvalue_yaw) false false)))

(event `self.IsDead`
  (`PrimitiveComponent.SetCollisionEnabled` (`self.CapsuleComponent`) "NoCollision")
  (`PrimitiveComponent.SetSimulatePhysics` (`self.Mesh`) true)
  (`PrimitiveComponent.SetCollisionEnabled` (`self.Mesh`) "PhysicsOnly"))

(fn `UserConstructionScript`
  (`parent.UserConstructionScript`)
  (`SceneComponent.K2_AttachToComponent` (`self.ArmHitbox`) (`self.Mesh`) "Arm" "KeepRelative" "KeepRelative" "KeepRelative" true)
  (`PrimitiveComponent.SetCollisionEnabled` (`self.ArmHitbox`) "NoCollision"))