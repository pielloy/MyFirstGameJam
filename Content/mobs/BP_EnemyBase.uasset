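; Base enemy Blueprint that handles taking damage, floating damage numbers and the death trigger.
; BeginPlay caches the DamageNumbers widget from the DamageText component.
; HitEnemy plays combat text and subtracts health until it is depleted, then sets IsDying to block further hits, calls IsDead and prints a debug string.
; IsDead is an empty event here, so the base has no death behavior of its own.
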(event `self.ReceiveBeginPlay`
  (bind _asdamage_numbers (cast `/Game/Widgets/DamageNumbers` (`WidgetComponent.GetUserWidgetObject` (`self.DamageText`))))
  (set `self.W_DamageText` _asdamage_numbers))

(event `self.ReceiveActorBeginOverlap`
  (params (OtherActor :type "Actor Object Reference")))

(event `self.ReceiveTick`
  (params (DeltaSeconds :type "Float (single-precision)")))

(event `/Game/mobs/Interface_EnemyDamagable.HitEnemy`
  (params (Damage :type "Float (single-precision)"))
  (if (not (`self.isDying?`))
    (`/Game/Widgets/DamageNumbers.PlayCombatText` (`self.W_DamageText`) Damage)
    (bind _output_get (set `self.EnemyHealth` (- (`self.EnemyHealth`) Damage)))
    (if (<= _output_get 0.0)
      (set `self.isDying?` true)
      (`self.IsDead`)
      (`KismetSystemLibrary.PrintString` "Hello"))))

(event `IsDead`)

(fn `UserConstructionScript`)