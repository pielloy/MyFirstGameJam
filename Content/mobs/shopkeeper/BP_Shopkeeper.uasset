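; BP_Shopkeeper is an interactable shopkeeper that shows an interact prompt and opens the player's shop UI.
; Detection events play the appear and disappear calls on its WBP_InteractShop widget.
; Interaction shows the cursor, switches to UI-only input, focuses the BP_Character widget, reveals its Shop panel and passes itself in as that panel's Shopkeeper.
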(event `self.OnDetect`
  (bind _aswbp_interact_shop (cast `/Game/mobs/shopkeeper/widgets/WBP_InteractShop` (`WidgetComponent.GetWidget` (`self.Widget`))))
  (`/Game/mobs/shopkeeper/widgets/WBP_InteractShop.OnApear` _aswbp_interact_shop))

(event `self.NotDetect`
  (bind _aswbp_interact_shop (cast `/Game/mobs/shopkeeper/widgets/WBP_InteractShop` (`WidgetComponent.GetWidget` (`self.Widget`))))
  (`/Game/mobs/shopkeeper/widgets/WBP_InteractShop.OnDisapear` _aswbp_interact_shop))

(event `self.IsInteractedWith`
  (bind _returnvalue (`GameplayStatics.GetPlayerController` 0))
  (set `PlayerController.bShowMouseCursor` true _returnvalue)
  (`WidgetBlueprintLibrary.SetInputMode_UIOnlyEx` _returnvalue null)
  (bind _asbp_character (cast `/Game/mobs/character/BP_Character` (`GameplayStatics.GetPlayerCharacter` 0)))
  (bind _widget (`/Game/mobs/character/BP_Character.Widget` _asbp_character))
  (`Widget.SetFocus` _widget)
  (bind _shop (`/Game/Widgets/inGame/WBP_InGame.Shop` _widget))
  (`Widget.SetVisibility` _shop "Visible")
  (set `/Game/mobs/shopkeeper/widgets/WBP_Shop.Shopkeeper` self _shop))

(fn `UserConstructionScript`)