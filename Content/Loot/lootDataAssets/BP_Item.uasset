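; BP_Item is a loot item Blueprint that carries stat values such as health, armor, damage and luck, plus a cheat-death flag.
; GetItemText builds its description by appending per-stat strings through a Text helper, with SoulsMultiplier truncated to three decimals and blank when zero.
; GenerateOnFloorItem takes a position but has an empty body.
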(fn `generateOnFloorItem`
  (params (Position :type "Vector Structure")))

(fn `getItemText`
  (returns (Text :type Text))
  (bind _soulsmultiplier (`self.SoulsMultiplier`))
  (return (`KismetTextLibrary.Conv_StringToText` (`KismetStringLibrary.Concat_StrStr` (`self.Text` "Health" (`self.Health`)) (`self.Text` "Armor" (`self.Armor`)) (`self.Text` "Damage" (`self.Damage`)) (`self.Text` "Parry damage" (`self.ParryDamage`)) (`self.Text` "Speed" (`self.Speed`)) (`self.Text` "Luck" (`self.luck`)) (`self.Text` "SoulsCapacity" (`self.SoulsCapacity`)) (`KismetMathLibrary.SelectString` "" (`KismetStringLibrary.Concat_StrStr` "SoulsMultiplier" ": " (`KismetStringLibrary.Conv_DoubleToString` (/ (`KismetMathLibrary.Conv_IntToDouble` (`KismetMathLibrary.FFloor` (* _soulsmultiplier 1000.0))) 1000.0)) " \n") (== _soulsmultiplier 0.0)) (`KismetMathLibrary.SelectString` "Cheat death" "" (`self.cheatDeath`))))))