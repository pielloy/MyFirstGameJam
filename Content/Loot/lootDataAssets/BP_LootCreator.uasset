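; BP_LootCreator picks luck-weighted loot and builds item instances with randomized stats.
; GetRandomLoot shifts base tier chances by Luck, then returns a random Pathetic, Decent, Epic or Enchanted entry from ItemsDataAsset.
; The first two tier checks roll separately, while the Epic check compares zero instead of a roll, so Enchanted needs a non-positive threshold sum.
; GenerateRandomLoot constructs a BP_Item, rolling stats within supplied modifier ranges and copying fixed properties.
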(fn GetRandomLoot
  (params (luck :type Float%20%28single-precision%29))
  (bind _returnvalue (Math|Random|RandomFloatinRange 0.0 1e+02))
  (bind _returnvalue_2 (|(BasePourcent+((luck*dif_afterLuck)/100)) 6e+01 luck -58.0))
  (bind _returnvalue_3 (|(BasePourcent+((luck*dif_afterLuck)/100)) 3e+01 luck -2e+01))
  (bind _itemsdataasset (Variables|Default|GetItemsDataAsset))
  (bind _itemsdataasset_2 (Variables|Default|GetItemsDataAsset))
  (bind _itemsdataasset_3 (Variables|Default|GetItemsDataAsset))
  (bind _itemsdataasset_4 (Variables|Default|GetItemsDataAsset))
  (bind _returnvalue_4 (+ _returnvalue_3 _returnvalue_2))
  (bind _decent (Variables|/Game/Loot/lootDataAssets/BP_LootSave.BP_LootSave_C|GetDecent _itemsdataasset_3))
  (bind _pathetic (Variables|/Game/Loot/lootDataAssets/BP_LootSave.BP_LootSave_C|GetPathetic _itemsdataasset_2))
  (bind _enchanted (Variables|/Game/Loot/lootDataAssets/BP_LootSave.BP_LootSave_C|GetEnchanted _itemsdataasset))
  (bind _epic (Variables|/Game/Loot/lootDataAssets/BP_LootSave.BP_LootSave_C|GetEpic _itemsdataasset_4))
  (if (< _returnvalue _returnvalue_2)
    (return (Utilities|Array|Get(acopy) _pathetic (Math|Random|RandomIntegerinRange 0 (- (Utilities|Array|Length _pathetic) 1))))
    (elif (< _returnvalue _returnvalue_4)
      (return (Utilities|Array|Get(acopy) _decent (Math|Random|RandomIntegerinRange 0 (- (Utilities|Array|Length _decent) 1))))
      (elif (< 0.0 (+ (|(BasePourcent+((luck*dif_afterLuck)/100)) 18.0 luck 22.0) _returnvalue_4))
        (return (Utilities|Array|Get(acopy) _epic (Math|Random|RandomIntegerinRange 0 (- (Utilities|Array|Length _epic) 1))))
        (else
          (return (Utilities|Array|Get(acopy) _enchanted (Math|Random|RandomIntegerinRange 0 (- (Utilities|Array|Length _enchanted) 1)))))))))

(fn GenerateRandomLoot
  (params (Luck :type BP%20Loot%20Info%20Object%20Reference))
  (bind _speedmodifier (Variables|/Game/Loot/lootDataAssets/BP_LootInfo.BP_LootInfo_C|GetSpeedModifier Luck))
  (bind _damagemodifier (Variables|/Game/Loot/lootDataAssets/BP_LootInfo.BP_LootInfo_C|GetDamageModifier Luck))
  (bind _parrytimemodifier (Variables|/Game/Loot/lootDataAssets/BP_LootInfo.BP_LootInfo_C|GetParryTimeModifier Luck))
  (bind _bartermodifier (Variables|/Game/Loot/lootDataAssets/BP_LootInfo.BP_LootInfo_C|GetBarterModifier Luck))
  (bind _luckmodifier (Variables|/Game/Loot/lootDataAssets/BP_LootInfo.BP_LootInfo_C|GetLuckModifier Luck))
  (bind _returnvalue (Game|ConstructObjectfromClass "/Game/Loot/lootDataAssets/BP_Item.BP_Item_C" self))
  (Variables|/Game/Loot/lootDataAssets/BP_Item.BP_Item_C|Setspeed _returnvalue (Math|Random|RandomFloatinRange (.x _speedmodifier) (.y _speedmodifier)))
  (Variables|/Game/Loot/lootDataAssets/BP_Item.BP_Item_C|Setdamage _returnvalue (Math|Random|RandomFloatinRange (.x _damagemodifier) (.y _damagemodifier)))
  (Variables|/Game/Loot/lootDataAssets/BP_Item.BP_Item_C|SetparryTime _returnvalue (Math|Random|RandomFloatinRange (.x _parrytimemodifier) (.y _parrytimemodifier)))
  (Variables|/Game/Loot/lootDataAssets/BP_Item.BP_Item_C|Setbarter _returnvalue (Math|Random|RandomFloatinRange (.x _bartermodifier) (.y _bartermodifier)))
  (Variables|/Game/Loot/lootDataAssets/BP_Item.BP_Item_C|Setluck _returnvalue (Math|Random|RandomFloatinRange (.x _luckmodifier) (.y _luckmodifier)))
  (Variables|/Game/Loot/lootDataAssets/BP_Item.BP_Item_C|SetcheatDeath _returnvalue (Variables|/Game/Loot/lootDataAssets/BP_LootInfo.BP_LootInfo_C|GetCheatDeath Luck))
  (Variables|/Game/Loot/lootDataAssets/BP_Item.BP_Item_C|Setrarity _returnvalue (Variables|/Game/Loot/lootDataAssets/BP_LootInfo.BP_LootInfo_C|GetRarity Luck))
  (Variables|/Game/Loot/lootDataAssets/BP_Item.BP_Item_C|SetmodifierType _returnvalue (Variables|/Game/Loot/lootDataAssets/BP_LootInfo.BP_LootInfo_C|GetModifierTypes Luck))
  (Variables|/Game/Loot/lootDataAssets/BP_Item.BP_Item_C|Setprice _returnvalue (Variables|/Game/Loot/lootDataAssets/BP_LootInfo.BP_LootInfo_C|GetPrice Luck))
  (return _returnvalue))