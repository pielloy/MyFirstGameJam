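; BP_ItemOnFloor is a loot pickup that adds its ItemData to the player character when interacted with, then destroys itself.
; Detection events play appear and disappear animations on its interact text widget.
; ChangeColorByRarity tints a dynamic material on the sphere and the Niagara effect for one of four rarities.
; BeginPlay always passes Enchanted, so the color does not follow the item data.
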(event `self.ReceiveBeginPlay`
  (`self.changeColorByRarity` "NewEnumerator3")
  (set `self.W_InteractText` (cast `/Game/Widgets/InteractableWidget` (`WidgetComponent.GetUserWidgetObject` (`self.InteractText`)) :!pure true)))

(event `self.IsInteractedWith`
  (bind _asbp_character (cast `/Game/mobs/character/BP_Character` (`GameplayStatics.GetPlayerPawn` 0)))
  (`/Game/mobs/character/BP_Character.addItem` _asbp_character (`self.itemData`))
  (`self.K2_DestroyActor`))

(event `OnDetect`
  (`/Game/Widgets/InteractableWidget.PlayInteractTextAppear` (`self.W_InteractText`)))

(event `NotDetect`
  (`/Game/Widgets/InteractableWidget.PlayInteractTextDissappear` (`self.W_InteractText`)))

(fn `changeColorByRarity`
  (params (Rarity :type "/Game/Loot/lootDataAssets/E_ItemRarity Enum" :default "NewEnumerator0"))
  (bind _niagara (`self.Niagara`))
  (bind _returnvalue (`PrimitiveComponent.CreateDynamicMaterialInstance` (`self.Sphere1`) 0 "/Game/Loot/lootDataAssets/MI_FloorItem.MI_FloorItem" "None"))
  (switch `/Game/Loot/lootDataAssets/E_ItemRarity` Rarity
    (:`NewEnumerator0`
      (`MaterialInstanceDynamic.SetVectorParameterValue` _returnvalue "Color" (struct :`R` 1.0 :`G` 1.0 :`B` 1.0 :`A` 1.0))
      (`FXSystemComponent.SetColorParameter` _niagara "Color" (struct :`R` 1.0 :`G` 1.0 :`B` 1.0 :`A` 1.0)))
    (:`NewEnumerator1`
      (`MaterialInstanceDynamic.SetVectorParameterValue` _returnvalue "Color" (struct :`R` 0.09217 :`G` 1.0 :`A` 1.0))
      (`FXSystemComponent.SetColorParameter` _niagara "Color" (struct :`R` 0.090842 :`G` 1.0 :`A` 1.0)))
    (:`NewEnumerator2`
      (`MaterialInstanceDynamic.SetVectorParameterValue` _returnvalue "Color" (struct :`R` 0.781339 :`B` 1.0 :`A` 1.0))
      (`FXSystemComponent.SetColorParameter` _niagara "Color" (struct :`R` 0.783538 :`B` 1.0 :`A` 1.0)))
    (:`NewEnumerator3`
      (`MaterialInstanceDynamic.SetVectorParameterValue` _returnvalue "Color" (struct :`R` 1.0 :`G` 0.872163 :`A` 1.0))
      (`FXSystemComponent.SetColorParameter` _niagara "Color" (struct :`R` 91.573097 :`G` 100.0 :`A` 1.0)))))

(fn `UserConstructionScript`)