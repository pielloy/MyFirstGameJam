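; BP_Map procedurally generates a maze of connected rooms with a matching minimap.
; The construction script fills a grid with BP_Tile objects, then links them through a shuffled recursive depth-first search from the origin.
; On BeginPlay, each tile's value indexes a 16-entry mesh and rotation table to spawn a BP_room.
; Each room gets a WBP_MiniMap tile, with the origin tile shown and highlighted.
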(event EventBeginPlay
  (bind _returnvalue (UserInterface|CreateWidget "/Game/map/minimap/WBP_MiniMap.WBP_MiniMap_C"))
  (bind _output_get (Variables|Default|Setwidget _returnvalue))
  (UserInterface|Viewport|AddtoViewport _output_get 0)
  (for (_array_element _array_index) (Variables|Default|GetMap)
    (for (_array_element_2 _array_index_2) (.row _array_element)
      (bind _value (Default|GetValue _array_element_2))
      (|SpawnTile_2 _value (Math|Vector2D|MakeVector2D (Math|Conversions|ToFloat(Integer) _array_index_2) (Math|Conversions|ToFloat(Integer) _array_index)) (Math|Conversions|ToFloat(Integer) _array_index_2) (Math|Conversions|ToFloat(Integer) _array_index)))))

(event Collision|EventActorBeginOverlap
  (params (OtherActor :type Actor%20Object%20Reference)))

(event EventTick
  (params (DeltaSeconds :type Float%20%28single-precision%29)))

(fn ConstructionScript
  (bind _map (Variables|Default|GetMap))
  (bind _size (Variables|Default|Getsize))
  ;[1 0.6269 0] Generate BP_Tile
  (for _index (range 0 (Math|Float|Truncate (.y _size)))
    (Utilities|Array|Add _map (Utilities|Struct|MakeST_Row))
    (for _index_2 (range 0 (Math|Float|Truncate (.x _size)))
      (bind _returnvalue (Game|ConstructObjectfromClass "/Game/map/BP_Tile.BP_Tile_C" self))
      (Variables|/Game/map/BP_Tile.BP_Tile_C|Setpos _returnvalue (Math|Vector2D|MakeVector2D (Math|Conversions|ToFloat(Integer) _index_2) (Math|Conversions|ToFloat(Integer) _index)))
      (Utilities|Array|Add (.row (Utilities|Array|Get(acopy) _map _index)) _returnvalue)))
  (CallFunction|Recursive)
  (Variables|Default|SettypeTiles (Utilities|Array|MakeArray (Utilities|Struct|MakeST_TypeTyle "/Game/map/mesh/tileZeroWay.tileZeroWay" 0.0) (Utilities|Struct|MakeST_TypeTyle "/Game/map/mesh/tileOneWay.tileOneWay" 9e+01) (Utilities|Struct|MakeST_TypeTyle "/Game/map/mesh/tileOneWay.tileOneWay" 1.8e+02) (Utilities|Struct|MakeST_TypeTyle "/Game/map/mesh/tileCorner.tileCorner" 0.0) (Utilities|Struct|MakeST_TypeTyle "/Game/map/mesh/tileOneWay.tileOneWay" 0.0) (Utilities|Struct|MakeST_TypeTyle "/Game/map/mesh/tileCorner.tileCorner" -9e+01) (Utilities|Struct|MakeST_TypeTyle "/Game/map/mesh/tileTwoWay.tileTwoWay" 0.0) (Utilities|Struct|MakeST_TypeTyle "/Game/map/mesh/tileThreeWay.tileThreeWay" -9e+01) (Utilities|Struct|MakeST_TypeTyle "/Game/map/mesh/tileOneWay.tileOneWay" -9e+01) (Utilities|Struct|MakeST_TypeTyle "/Game/map/mesh/tileTwoWay.tileTwoWay" 9e+01) (Utilities|Struct|MakeST_TypeTyle "/Game/map/mesh/tileCorner.tileCorner" 9e+01) (Utilities|Struct|MakeST_TypeTyle "/Game/map/mesh/tileThreeWay.tileThreeWay" 0.0) (Utilities|Struct|MakeST_TypeTyle "/Game/map/mesh/tileCorner.tileCorner" 1.8e+02) (Utilities|Struct|MakeST_TypeTyle "/Game/map/mesh/tileThreeWay.tileThreeWay" 1.8e+02) (Utilities|Struct|MakeST_TypeTyle "/Game/map/mesh/tileThreeWay.tileThreeWay" 9e+01) (Utilities|Struct|MakeST_TypeTyle 0 0.0))))

(fn Recursive
  (params (pos :type Vector%202D%20Structure) (exept :type Vector%202D%20Structure))
  (bind _output_get (LocalVariables|SetTest (Utilities|Array|MakeArray "(X=1.000000,Y=0.000000)" "(X=0.000000,Y=1.000000)" "(X=-1.000000,Y=0.000000)" "(X=0.000000,Y=-1.000000)")))
  (Utilities|Array|Shuffle _output_get)
  (for (_array_element _array_index) (LocalVariables|GetTest)
    (if (not (Math|Vector|Equal(Vector) (Utilities|Array|Get(acopy) (LocalVariables|GetTest) _array_index) exept 0.0001))
      (|TestIfNotOutside (- (.x pos) (.x _array_element)) (- (.y pos) (.y _array_element)) (- (.x pos) (.x _array_element)) (- (.y pos) (.y _array_element))
        (:else
          (bind _isfilled_ (Default|IsFilled (Utilities|GetTile (- (.x pos) (.x _array_element)) (- (.y pos) (.y _array_element)))))
          (if (not _isfilled_)
            (|SetDirection (Utilities|GetTile (.x pos) (.y pos)) _array_index (Utilities|GetTile (- (.x pos) (.x _array_element)) (- (.y pos) (.y _array_element))) (LocalVariables|GetTest)
              (:Output
                (CallFunction|Recursive (Math|Vector2D|MakeVector2D (- (.x pos) (.x _array_element)) (- (.y pos) (.y _array_element))) (Math|Vector2D|MakeVector2D (* (.x (Utilities|Array|Get(acopy) (LocalVariables|GetTest) _array_index)) -1.0) (* (.y (Utilities|Array|Get(acopy) (LocalVariables|GetTest) _array_index)) -1.0)))))))))))