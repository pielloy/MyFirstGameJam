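; BP_RoomType describes a map room by which of its four sides connect to other rooms.
; GetValue packs the bottom, right, left and top connection flags into an integer bitmask, bottom as the lowest bit and top as the highest.
; IsFilled reports true when at least one side is connected.
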(fn `getValue`
  (returns (Value :type Integer))
  (return (`KismetMathLibrary.FTrunc` (+ (`KismetMathLibrary.SelectFloat` (`KismetMathLibrary.MultiplyMultiply_FloatFloat` 2.0) 0.0 (`self.isConnectedBottom?`)) (`KismetMathLibrary.SelectFloat` (`KismetMathLibrary.MultiplyMultiply_FloatFloat` 2.0 1.0) 0.0 (`self.isConnectedRight?`)) (`KismetMathLibrary.SelectFloat` (`KismetMathLibrary.MultiplyMultiply_FloatFloat` 2.0 2.0) 0.0 (`self.isConnectedLeft`)) (`KismetMathLibrary.SelectFloat` (`KismetMathLibrary.MultiplyMultiply_FloatFloat` 2.0 3.0) 0.0 (`self.isConnectedTop?`))))))

(fn `isFilled`
  (returns (connected :type Boolean))
  (return (or (`self.isConnectedTop?`) (`self.isConnectedBottom?`) (`self.isConnectedLeft`) (`self.isConnectedRight?`))))