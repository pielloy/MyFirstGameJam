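; BP_Tile is a map tile that tracks whether it connects on its top, left, right and bottom sides.
; IsFilled reports whether any side is connected.
; GetValue packs the four flags into a bitmask by summing BaseTwo results, with top as the highest bit and bottom as the lowest.
; BaseTwo contains the bool-times-power-of-two math for each bit.
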(fn `getValue`
  (returns (value :type Integer))
  (return (+ (`self.BaseTwo` (`self.isConnectedTop?`) 3.0) (`self.BaseTwo` (`self.isConnectedLeft?`) 2.0) (`self.BaseTwo` (`self.isConnectedRight?`) 1.0) (`self.BaseTwo` (`self.isConnectedBottom?`)))))

(fn `isFilled`
  (returns (`isFilled?` :type Boolean))
  (locals (nbrTest :type Integer))
  (return (or (`self.isConnectedTop?`) (`self.isConnectedLeft?`) (`self.isConnectedRight?`) (`self.isConnectedBottom?`))))