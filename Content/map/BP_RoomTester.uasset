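; BP_RoomTester is an actor that builds a single room from RoomData, apparently for testing room layouts.
; On BeginPlay it spawns the room's actor at its stored offset, then a random class from the Enemys list at each spawner location, all offset from the tester's position.
; The construction script adds a rotated arrow component at each spawner location, so spawn points can be previewed in the editor.
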(event `self.ReceiveBeginPlay`
  (bind _roomdata (`self.RoomData`))
  (bind _enemys (`/Game/map/utils/BP_EnemySave.Enemys` (`self.Enemys`)))
  (if (!= _roomdata null)
    (`|SpawnActorFromClass` (`/Game/map/utils/BP_RoomContent.Actor` _roomdata) (`KismetMathLibrary.MakeTransform` (+ (`self.K2_GetActorLocation`) (`/Game/map/utils/BP_RoomContent.ActorLocation` _roomdata))) "Undefined" "OverrideRootScale" null null)
    (for _array_element (`/Game/map/utils/BP_RoomContent.SpawnerLocation` _roomdata)
      (`|SpawnActorFromClass` (`|GetArrayItem` _enemys (`KismetMathLibrary.RandomIntegerInRange` 0 (- (`KismetArrayLibrary.Array_Length` _enemys) 1))) (`KismetMathLibrary.MakeTransform` (+ _array_element (`self.K2_GetActorLocation`))) "Undefined" "OverrideRootScale" null null))))

(fn `UserConstructionScript`
  (bind _roomdata (`self.RoomData`))
  (if (!= _roomdata null)
    (for _array_element (`/Game/map/utils/BP_RoomContent.SpawnerLocation` _roomdata)
      (`AddComponent|NODE_AddArrowComponent-0` :`RelativeTransform` (`KismetMathLibrary.MakeTransform` _array_element (struct :`Pitch` -90.0))))))